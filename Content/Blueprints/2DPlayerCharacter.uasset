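; Player character for a 2D side-scroller that runs along the X axis, jumps, dies and respawns.
; Each tick picks a death, jump, move or idle flipbook and turns the controller yaw to face the travel direction, keeping the last input direction when still.
; Any damage kills: movement is disabled until just before the death animation ends, then the character returns to its BeginPlay location.
; BeginPlay also creates the player HUD.
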(event Custom|Handle%20Animation
  (bind _sprite (Variables|Default|GetSprite))
  ;[0.15 0.15 0.15 0.5] Handle Animation
  (if (Variables|Default|GetisDead)
    (Sprite|SetFlipbook (Variables|Default|GetSprite) (Variables|Default|GetplayerDeathAnimation))
    (elif (AI|Components|NavMovement|IsFalling (Variables|Character|GetCharacterMovement))
      (Sprite|SetFlipbook _sprite "/Game/Assets/kenney_pixel-platformer/Tiles/Characters/Jumping.Jumping")
      (else
        (Sprite|SetFlipbook _sprite (select (> (Math|Vector|VectorLength (Variables|/Script/Engine.MovementComponent|GetVelocity (Variables|Character|GetCharacterMovement))) 0.0) "/Game/Assets/kenney_pixel-platformer/Tiles/Characters/Moving.Moving" "/Game/Assets/kenney_pixel-platformer/Tiles/Characters/Idle.Idle"))))))

(event Custom|HandleRotation
  ;[0.15 0.15 0.15 0.5] Handle Rotation
  (Math|Float|CompareFloat (.x (Variables|/Script/Engine.MovementComponent|GetVelocity (Variables|Character|GetCharacterMovement))) 0.0
    (:>
      (Pawn|SetControlRotation (Pawn|GetController) (Math|Rotator|MakeRotator 0.0 0.0 1.8e+02) :!label _label))
    (:==
      (if (Variables|Default|GetisMovingRight?)
        (goto _label)
        (else
          (Pawn|SetControlRotation (Pawn|GetController) (Math|Rotator|MakeRotator 0.0 0.0 0.0) :!label _label_2))))
    (:<
      (goto _label_2))))

(event Custom|RespawnPlayerCharacter
  ;[0.15 0.15 0.15 0.5] Handle Player Character Respawn
  (Transformation|SetActorLocationAndRotation (Variables|Default|GetrespawnLocation) "0, 0, 0")
  (Variables|Default|SetisDead false)
  (Components|Activation|SetActive (Variables|Character|GetCharacterMovement) true false))

(event EventTick
  (params (DeltaSeconds :type Float%20%28single-precision%29))
  ;[0.15 0.15 0.15 0.5] Event Tick
  (CallFunction|HandleAnimation)
  (CallFunction|HandleRotation))

(event Game|Damage|EventAnyDamage
  (params (Damage :type Float%20%28single-precision%29) (DamageType :type Damage%20Type%20Object%20Reference) (InstigatedBy :type Controller%20Object%20Reference) (DamageCauser :type Actor%20Object%20Reference))
  ;[0.15 0.15 0.15 0.5] Handle Damage
  (Variables|Default|SetisDead true)
  (Components|Activation|SetActive (Variables|Character|GetCharacterMovement) false false)
  (Utilities|FlowControl|Delay (- (Class|PaperFlipbook|GetTotalDuration (Variables|Default|GetplayerDeathAnimation)) 0.1))
  (CallFunction|RespawnPlayerCharacter))

(event EventBeginPlay
  ;[0.15 0.15 0.15 0.5] Event Begin Play
  (Variables|Default|SetrespawnLocation (Transformation|GetActorLocation))
  (bind _returnvalue (UserInterface|CreateWidget "/Game/UI/PlayerHUD.PlayerHUD_C"))
  (bind _output_get (Variables|Default|SetplayerHUD _returnvalue))
  (UserInterface|Viewport|AddtoViewport _output_get 0))

(event Input|ActionEvents|InputActionJump
  (params (Key :type Key%20Structure :default "None"))
  ;[0.15 0.15 0.15 0.5] Handle Jumping
  (:Pressed
    (Character|Jump))
  (:Released
    (Character|StopJumping)))

(event Input|AxisEvents|InputAxisMoveRight
  (params (AxisValue :type Float%20%28single-precision%29))
  ;[0.15 0.15 0.15 0.5] Handle Movement
  (if (> AxisValue 0.0)
    (Variables|Default|SetisMovingRight? true)
    (elif (< AxisValue 0.0)
      (Variables|Default|SetisMovingRight? false)))
  (Pawn|Input|AddMovementInput "1.000000,0.000000,0.000000" AxisValue false))

(fn ConstructionScript)